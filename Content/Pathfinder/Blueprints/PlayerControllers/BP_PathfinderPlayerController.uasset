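; Player controller for Pathfinder that toggles the pause menu on the P key.
; Pausing creates W_PauseMenu, adds it to the viewport, focuses it in UI-only input mode and shows the cursor.
; Unpausing finds and removes every top-level W_PauseMenu instead of storing a reference, then restores game-only input and hides the cursor.
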(event EventBeginPlay)

(event EventTick
  (params (DeltaSeconds :type Float%20%28single-precision%29)))

(event Input|KeyboardEvents|P
  (params (Key :type Key%20Structure :default "None"))
  (:Pressed
    (if (Game|IsGamePaused)
      (Game|SetGamePaused false)
      (bind _foundwidgets (Widget|GetAllWidgetsOfClass "/Game/Pathfinder/UI/W_PauseMenu.W_PauseMenu_C" true))
      (for _array_element _foundwidgets
        (Widget|RemovefromParent _array_element))
      (Input|SetInputModeGameOnly self false)
      (Variables|Default|SetbShowMouseCursor false)
      (else
        (Game|SetGamePaused true)
        (bind _returnvalue (UserInterface|CreateWidget "/Game/Pathfinder/UI/W_PauseMenu.W_PauseMenu_C"))
        (UserInterface|Viewport|AddtoViewport _returnvalue 0)
        (Input|SetInputModeUIOnly self _returnvalue "DoNotLock" false)
        (Variables|Default|SetbShowMouseCursor true)))))

(fn ConstructionScript)